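; Enemy AI character that senses the player and can kill them with a melee attack.
; Perception updates feed the AI controller's blackboard: sight sets Player, other senses set CheckLoc, and any failed stimulus clears Player.
; Attack plays the enemy montage.
; AttackTrace sphere-traces pawns at the right-hand socket with debug drawing, destroying a hit ThirdPersonCharacter unless the game instance's GodMode is on.
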(event OnTargetPerceptionUpdated(AIPerception)
  (params (Actor :type Actor%20Object%20Reference) (Stimulus :type AI%20Stimulus%20Structure))
  (if (.bSuccessfullySensed (Utilities|Struct|BreakAIStimulus Stimulus))
    (bind _output_get (Variables|Default|SetStimulus Stimulus))
    (bind _returnvalue (Class|AIPerceptionSystem|GetSenseClassforStimulus _output_get))
    (if (== _returnvalue "/Script/AIModule.AISense_Sight")
      (Utilities|Casting|CastToThirdPersonCharacter Actor)
      (AI|Components|Blackboard|SetValueasObject (AI|GetBlackboard (Variables|Default|GetAIController)) (Utilities|Name|MakeLiteralName "Player") Actor)
      (else
        (AI|Components|Blackboard|SetValueasVector (AI|GetBlackboard (Variables|Default|GetAIController)) (Utilities|Name|MakeLiteralName "CheckLoc") (.stimuluslocation (Variables|Default|GetStimulus)))))
    (else
      (AI|Components|Blackboard|ClearValue (AI|GetBlackboard (Variables|Default|GetAIController)) (Utilities|Name|MakeLiteralName "Player")))))

(event EventBeginPlay
  (Variables|Default|SetAIController (AI|GetAIController self)))

(fn ConstructionScript)

(fn Attack
  (Animation|PlayAnimMontage "/Game/AI/Asset/AnimMontage_Enemy.AnimMontage_Enemy" 1.0 "None"))

(fn AttackTrace
  (bind _mesh (Variables|Character|GetMesh))
  (bind _returnvalue (Transformation|GetSocketLocation _mesh "RightHand"))
  (bind _outhit (Collision|SphereTraceForObjects _returnvalue _returnvalue 2e+01 (Utilities|Array|MakeArray "ObjectTypeQuery3") false 0 "ForDuration"))
  (bind _asthird_person_character (Utilities|Casting|CastToThirdPersonCharacter (.HitActor (Collision|BreakHitResult _outhit))))
  (bind _asgam_instance_store_var (Utilities|Casting|CastToGamInstance_StoreVar (Game|GetGameInstance)))
  (if (not (Variables|/Game/Maps/GamInstance_StoreVar.GamInstance_StoreVar_C|GetGodMode _asgam_instance_store_var))
    (Actor|DestroyActor _asthird_person_character)))